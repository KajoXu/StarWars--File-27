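; BP_DoubleProjectile is a projectile actor with two projectile components that damage whatever they overlap.
; Each component's begin overlap applies a fixed amount of damage to the other actor, then destroys the whole actor.
; When IsDeflecting is set, the overlap clears that flag instead of destroying the actor, so it survives that hit after still dealing damage.
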(event OnComponentBeginOverlap(Projectile1)
  (params (OverlappedComponent :type Primitive%20Component%20Object%20Reference) (OtherActor :type Actor%20Object%20Reference) (OtherComp :type Primitive%20Component%20Object%20Reference) (OtherBodyIndex :type Integer) (bFromSweep :type Boolean) (SweepResult :type Hit%20Result%20Structure%20%28by%20ref%29))
  (Game|Damage|ApplyDamage OtherActor 2e+01 0 self)
  (if (Variables|Default|GetisDeflecting?)
    (Variables|Default|SetisDeflecting? false)
    (else
      (Actor|DestroyActor))))

(event OnComponentBeginOverlap(Projectile)
  (params (OverlappedComponent :type Primitive%20Component%20Object%20Reference) (OtherActor :type Actor%20Object%20Reference) (OtherComp :type Primitive%20Component%20Object%20Reference) (OtherBodyIndex :type Integer) (bFromSweep :type Boolean) (SweepResult :type Hit%20Result%20Structure%20%28by%20ref%29))
  (Game|Damage|ApplyDamage OtherActor 2e+01 0 self)
  (if (Variables|Default|GetisDeflecting?)
    (Variables|Default|SetisDeflecting? false)
    (else
      (Actor|DestroyActor))))

(fn ConstructionScript)