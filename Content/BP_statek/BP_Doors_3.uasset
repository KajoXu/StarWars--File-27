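; BP_Doors_3 is a door pair that opens once three enemies have died.
; The first overlap of BP_twi_lek with its box sets the enemy counter, and each HesDead call decrements it.
; At zero, a timeline slides both door meshes by vector lerp and raises the BP_spawn1 actor once.
; SpawnEnemies spawns B1 and B2 droids at spawn points but is not called within this Blueprint.
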(event OnComponentBeginOverlap(Box)
  (params (OverlappedComponent :type Primitive%20Component%20Object%20Reference) (OtherActor :type Actor%20Object%20Reference) (OtherComp :type Primitive%20Component%20Object%20Reference) (OtherBodyIndex :type Integer) (bFromSweep :type Boolean) (SweepResult :type Hit%20Result%20Structure%20%28by%20ref%29))
  (if (== (Utilities|GetClass OtherActor) "/Game/Characters/twi_lek/BP_twi_lek.BP_twi_lek_C")
    (Utilities|FlowControl|DoOnce false
      (:Completed
        (Variables|Default|SetEnemies%20Left 3)))))

(event EventHesDead
  (bind _result (Math|Integer|DecrementInt (Variables|Default|GetEnemies%20Left))
    (:%20%20
      (Variables|Default|SetEnemies%20Left _result)
      (if (== (Variables|Default|GetEnemies%20Left) 0)
        (bind _newtrack_0 (Timeline|Timeline_Doors Play)
          (:Update
            (Transformation|SetRelativeLocation (Variables|Default|Getdrzwi_drzwi_008) (Math|Vector|Lerp(Vector) (Variables|Default|Getoldr) (Variables|Default|Getnewr) _newtrack_0) false false)
            (Transformation|SetRelativeLocation (Variables|Default|Getdrzwi_drzwi_009) (Math|Vector|Lerp(Vector) (Variables|Default|Getoldl) (Variables|Default|Getnewl) _newtrack_0) false false)
            (Utilities|FlowControl|DoOnce false
              (:Completed
                (bind _returnvalue (Actor|GetActorOfClass "/Game/BP_statek/BP_spawn1.BP_spawn1_C"))
                (Transformation|SetActorLocation _returnvalue (+ (Transformation|GetActorLocation _returnvalue) "0,0,500.000000") false false)))))))))

(fn ConstructionScript)

(fn SpawnEnemies
  (bind _spawn_points (Variables|Default|GetSpawn%20Points))
  (AI|SpawnAIFromClass "/Game/Characters/AI_B2Droid/AI_B2Droid.AI_B2Droid_C" "/Game/Characters/AI_B2Droid/BT_B2Droid.BT_B2Droid" (Transformation|GetActorLocation (Utilities|Array|Get(acopy) _spawn_points)) "0, 0, 0" false 0)
  (AI|SpawnAIFromClass "/Game/Characters/AI_B1Droid/AI_B1Droid.AI_B1Droid_C" 0 (Transformation|GetActorLocation (Utilities|Array|Get(acopy) _spawn_points 1)) "0, 0, 0" false 0)
  (AI|SpawnAIFromClass "/Game/Characters/AI_B2Droid/AI_B2Droid.AI_B2Droid_C" "/Game/Characters/AI_B2Droid/BT_B2Droid.BT_B2Droid" (Transformation|GetActorLocation (Utilities|Array|Get(acopy) _spawn_points 2)) "0, 0, 0" false 0))