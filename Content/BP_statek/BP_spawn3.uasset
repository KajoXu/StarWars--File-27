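; BP_spawn3 is a combat encounter trigger that locks the player in until the enemies are dead.
; The first BP_twi_lek overlap sets the enemy count, closes BP_Doors_7, starts DC_FightDirector and sends every AI_DroidCommandoController to fight.
; HesDead counts down deaths; at zero it reopens the doors and resets BP_spawn2 with RightDoors cleared.
; A SpawnEnemies function spawns B1 droids at spawn points but is not called here.
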(event OnComponentBeginOverlap(Box)
  (params (OverlappedComponent :type Primitive%20Component%20Object%20Reference) (OtherActor :type Actor%20Object%20Reference) (OtherComp :type Primitive%20Component%20Object%20Reference) (OtherBodyIndex :type Integer) (bFromSweep :type Boolean) (SweepResult :type Hit%20Result%20Structure%20%28by%20ref%29))
  (if (== (Utilities|GetClass OtherActor) "/Game/Characters/twi_lek/BP_twi_lek.BP_twi_lek_C")
    (Utilities|FlowControl|DoOnce false
      (:Completed
        (Variables|Default|SetEnemiesLeft 6)
        (Default|CloseDoors (Utilities|Array|Get(acopy) (stale EventBeginPlay _outactors_4)))
        (Default|StartFight (Utilities|Array|Get(acopy) (stale EventBeginPlay _outactors_5)))
        (for _array_element (stale EventBeginPlay _outactors_6)
          (Default|MovetoFight _array_element))))))

(event EventBeginPlay
  (bind _outactors (Actor|GetAllActorsOfClass "/Game/BP_statek/BP_spawn2.BP_spawn2_C"))
  (Variables|Default|Setspawn2%20REF (Utilities|Array|Get(acopy) _outactors))
  (bind _outactors_2 (Actor|GetAllActorsOfClass "/Game/BP_statek/BP_Doors_5.BP_Doors_5_C"))
  (Variables|Default|Setdoors5%20REF (Utilities|Array|Get(acopy) _outactors_2))
  (bind _outactors_3 (Actor|GetAllActorsOfClass "/Game/BP_statek/BP_Doors_6.BP_Doors_6_C"))
  (Variables|Default|Setdoors6%20REF (Utilities|Array|Get(acopy) _outactors_3))
  (bind _outactors_4 (Actor|GetAllActorsOfClass "/Game/BP_statek/BP_Doors_7.BP_Doors_7_C"))
  (bind _outactors_5 (Actor|GetAllActorsOfClass "/Game/Characters/AI_DroidCommando/DC_FightDirector.DC_FightDirector_C"))
  (bind _outactors_6 (Actor|GetAllActorsOfClass "/Game/Characters/AI_DroidCommando/AI_DroidCommandoController.AI_DroidCommandoController_C"))
  (Actor|GetAllActorsOfClass "/Game/Characters/AI_DroidCommando/AI_DroidCommando.AI_DroidCommando_C"))

(event EventHesDead
  (bind _spawn2_ref (Variables|Default|Getspawn2%20REF))
  (bind _result (Math|Integer|DecrementInt (Variables|Default|GetEnemiesLeft))
    (:%20%20
      (bind _output_get (Variables|Default|SetEnemiesLeft _result))
      (if (== _output_get 0)
        (Default|OpenDoors (Utilities|Array|Get(acopy) (stale EventBeginPlay _outactors_4)))
        (Variables|/Game/BP_statek/BP_spawn2.BP_spawn2_C|SetrightDoors _spawn2_ref false)
        (Default|ResetState _spawn2_ref)))))

(fn ConstructionScript)

(fn SpawnEnemies
  (bind _spawnpoints (Variables|Default|GetSpawnPoints))
  (bind _counter (Utilities|FlowControl|DoN (Utilities|Array|Length _spawnpoints))
    (:Exit
      (AI|SpawnAIFromClass "/Game/Characters/AI_B1Droid/AI_B1Droid.AI_B1Droid_C" 0 (Transformation|GetActorLocation (Utilities|Array|Get(acopy) _spawnpoints _counter)) "0, 0, 0" false 0))))