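; BP_Doors_8 is a double door tied to combat, opening when its enemy counter reaches zero or the boss dies.
; A timeline lerps both door meshes between stored positions and reverses to close them.
; BeginPlay caches the Magnaguard, its controller and BP_spawn2; boss death also resets that spawn's state and sets its FinalDoors flag.
; SpawnEnemies creates B1 and B2 droids at spawn points but is not called within this Blueprint.
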(event Custom|CloseDoors
  (bind _newtrack_0 (Timeline|Timeline_Doors Reverse)
    (:Update
      (Transformation|SetRelativeLocation (Variables|Default|Getdrzwi_drzwi_008) (Math|Vector|Lerp(Vector) (Variables|Default|Getoldr) (Variables|Default|Getnewr) _newtrack_0) false false)
      (Transformation|SetRelativeLocation (Variables|Default|Getdrzwi_drzwi_009) (Math|Vector|Lerp(Vector) (Variables|Default|Getoldl) (Variables|Default|Getnewl) _newtrack_0) false false))))

(event Custom|OpenDoors
  (bind _newtrack_0 (Timeline|Timeline_Doors Play)
    (:Update
      (Transformation|SetRelativeLocation (Variables|Default|Getdrzwi_drzwi_008) (Math|Vector|Lerp(Vector) (Variables|Default|Getoldr) (Variables|Default|Getnewr) _newtrack_0) false false)
      (Transformation|SetRelativeLocation (Variables|Default|Getdrzwi_drzwi_009) (Math|Vector|Lerp(Vector) (Variables|Default|Getoldl) (Variables|Default|Getnewl) _newtrack_0) false false))))

(event EventBeginPlay
  (bind _outactors (Actor|GetAllActorsOfClass "/Game/Characters/AI_Magnaguard/AI_Magnaguard.AI_Magnaguard_C"))
  (Variables|Default|Setig-100%20REF (Utilities|Array|Get(acopy) _outactors))
  (bind _outactors_2 (Actor|GetAllActorsOfClass "/Game/Characters/AI_Magnaguard/AI_MagnaguardController.AI_MagnaguardController_C"))
  (Variables|Default|Setig-100%20C%20REF (Utilities|Array|Get(acopy) _outactors_2))
  (bind _outactors_3 (Actor|GetAllActorsOfClass "/Game/BP_statek/BP_spawn2.BP_spawn2_C"))
  (Variables|Default|Setspawn2%20REF (Utilities|Array|Get(acopy) _outactors_3)))

(event EventHesDead
  (bind _result (Math|Integer|DecrementInt (Variables|Default|GetEnemies%20Left))
    (:%20%20
      (bind _output_get (Variables|Default|SetEnemies%20Left _result))
      (if (== _output_get 0)
        (CallFunction|OpenDoors)))))

(event EventBossIsDead
  (bind _spawn2_ref (Variables|Default|Getspawn2%20REF))
  (CallFunction|OpenDoors)
  (Default|ResetState _spawn2_ref)
  (Variables|/Game/BP_statek/BP_spawn2.BP_spawn2_C|SetfinalDoors? _spawn2_ref true))

(fn ConstructionScript)

(fn SpawnEnemies
  (bind _spawn_points (Variables|Default|GetSpawn%20Points))
  (AI|SpawnAIFromClass "/Game/Characters/AI_B2Droid/AI_B2Droid.AI_B2Droid_C" "/Game/Characters/AI_B2Droid/BT_B2Droid.BT_B2Droid" (Transformation|GetActorLocation (Utilities|Array|Get(acopy) _spawn_points)) "0, 0, 0" false 0)
  (AI|SpawnAIFromClass "/Game/Characters/AI_B1Droid/AI_B1Droid.AI_B1Droid_C" 0 (Transformation|GetActorLocation (Utilities|Array|Get(acopy) _spawn_points 1)) "0, 0, 0" false 0)
  (AI|SpawnAIFromClass "/Game/Characters/AI_B2Droid/AI_B2Droid.AI_B2Droid_C" "/Game/Characters/AI_B2Droid/BT_B2Droid.BT_B2Droid" (Transformation|GetActorLocation (Utilities|Array|Get(acopy) _spawn_points 2)) "0, 0, 0" false 0))