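; Wave manager actor that runs a four-wave droid encounter, triggered once by overlapping any of four start volumes.
; Each wave spawns B1 and B2 droids at preset spawn points and, after the first, activates placed Vultures.
; HesDead counts down remaining enemies, and EndWave starts the next wave after a short delay.
; Once the last wave is cleared, it sends CanGoToMessage to all BP_Doors and BP_spawn actors found at start.
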(event OnComponentBeginOverlap(StartWavePointForward)
  (params (OverlappedComponent :type Primitive%20Component%20Object%20Reference) (OtherActor :type Actor%20Object%20Reference) (OtherComp :type Primitive%20Component%20Object%20Reference) (OtherBodyIndex :type Integer) (bFromSweep :type Boolean) (SweepResult :type Hit%20Result%20Structure%20%28by%20ref%29))
  (Utilities|FlowControl|DoOnce false
    (:Completed
      (CallFunction|StartNewWave)
      (bind _outactors (Actor|GetAllActorsOfClass "/Game/BP_statek/BP_Doors.BP_Doors_C"))
      (bind _outactors_2 (Actor|GetAllActorsOfClass "/Game/BP_statek/BP_spawn.BP_spawn_C")))))

(event OnComponentBeginOverlap(StartWavePointBackward)
  (params (OverlappedComponent :type Primitive%20Component%20Object%20Reference) (OtherActor :type Actor%20Object%20Reference) (OtherComp :type Primitive%20Component%20Object%20Reference) (OtherBodyIndex :type Integer) (bFromSweep :type Boolean) (SweepResult :type Hit%20Result%20Structure%20%28by%20ref%29))
  (Utilities|FlowControl|DoOnce false
    (:Completed
      (CallFunction|StartNewWave)
      (bind _outactors (Actor|GetAllActorsOfClass "/Game/BP_statek/BP_Doors.BP_Doors_C"))
      (bind _outactors_2 (Actor|GetAllActorsOfClass "/Game/BP_statek/BP_spawn.BP_spawn_C")))))

(event OnComponentBeginOverlap(StartWavePointLeft)
  (params (OverlappedComponent :type Primitive%20Component%20Object%20Reference) (OtherActor :type Actor%20Object%20Reference) (OtherComp :type Primitive%20Component%20Object%20Reference) (OtherBodyIndex :type Integer) (bFromSweep :type Boolean) (SweepResult :type Hit%20Result%20Structure%20%28by%20ref%29))
  (Utilities|FlowControl|DoOnce false
    (:Completed
      (CallFunction|StartNewWave)
      (bind _outactors (Actor|GetAllActorsOfClass "/Game/BP_statek/BP_Doors.BP_Doors_C"))
      (bind _outactors_2 (Actor|GetAllActorsOfClass "/Game/BP_statek/BP_spawn.BP_spawn_C")))))

(event OnComponentBeginOverlap(StartWavePointRight)
  (params (OverlappedComponent :type Primitive%20Component%20Object%20Reference) (OtherActor :type Actor%20Object%20Reference) (OtherComp :type Primitive%20Component%20Object%20Reference) (OtherBodyIndex :type Integer) (bFromSweep :type Boolean) (SweepResult :type Hit%20Result%20Structure%20%28by%20ref%29))
  (Utilities|FlowControl|DoOnce false
    (:Completed
      (CallFunction|StartNewWave)
      (bind _outactors (Actor|GetAllActorsOfClass "/Game/BP_statek/BP_Doors.BP_Doors_C"))
      (bind _outactors_2 (Actor|GetAllActorsOfClass "/Game/BP_statek/BP_spawn.BP_spawn_C")))))

(event Custom|End%20Wave
  (bind _current_wave (Variables|Default|GetCurrent%20Wave))
  (bind _returnvalue (== _current_wave 5))
  (Utilities|FlowControl|Delay 1.0)
  (CallFunction|StartNewWave)
  (if _returnvalue
    (Class|BPICanGoto|CanGoto(Message) (stale OnComponentBeginOverlap(StartWavePointForward) _outactors) _returnvalue)
    (Class|BPICanGoto|CanGoto(Message) (stale OnComponentBeginOverlap(StartWavePointForward) _outactors_2) _returnvalue)))

(event EventHesDead
  (bind _result (Math|Integer|DecrementInt (Variables|Default|GetEnemies%20Left))
    (:%20%20
      (Variables|Default|SetEnemies%20Left _result)
      (if (== (Variables|Default|GetEnemies%20Left) 0)
        (CallFunction|EndWave)))))

(fn ConstructionScript)

(fn EnemiesforThirdWave
  (bind _spawn_points (Variables|Default|GetSpawn%20Points))
  (bind _vulture_spawn (Variables|Default|GetVulture%20Spawn))
  (AI|SpawnAIFromClass "/Game/Characters/AI_B1Droid/AI_B1Droid.AI_B1Droid_C" 0 (Transformation|GetActorLocation (Utilities|Array|Get(acopy) _spawn_points 7)) "0, 0, 0" false 0)
  (AI|SpawnAIFromClass "/Game/Characters/AI_B2Droid/AI_B2Droid.AI_B2Droid_C" "/Game/Characters/AI_B2Droid/BT_B2Droid.BT_B2Droid" (Transformation|GetActorLocation (Utilities|Array|Get(acopy) _spawn_points 8)) "0, 0, 0" false 0)
  (AI|SpawnAIFromClass "/Game/Characters/AI_B1Droid/AI_B1Droid.AI_B1Droid_C" 0 (Transformation|GetActorLocation (Utilities|Array|Get(acopy) _spawn_points 9)) "0, 0, 0" false 0)
  (AI|SpawnAIFromClass "/Game/Characters/AI_B1Droid/AI_B1Droid.AI_B1Droid_C" 0 (Transformation|GetActorLocation (Utilities|Array|Get(acopy) _spawn_points 10)) "0, 0, 0" false 0)
  (AI|SpawnAIFromClass "/Game/Characters/AI_B2Droid/AI_B2Droid.AI_B2Droid_C" "/Game/Characters/AI_B2Droid/BT_B2Droid.BT_B2Droid" (Transformation|GetActorLocation (Utilities|Array|Get(acopy) _spawn_points 11)) "0, 0, 0" false 0)
  (Default|StartAIBehaviour (Utilities|Array|Get(acopy) _vulture_spawn 1))
  (Default|StartAIBehaviour (Utilities|Array|Get(acopy) _vulture_spawn 2)))

(fn EnemiesforSecondWave
  (bind _spawn_points (Variables|Default|GetSpawn%20Points))
  (AI|SpawnAIFromClass "/Game/Characters/AI_B2Droid/AI_B2Droid.AI_B2Droid_C" "/Game/Characters/AI_B2Droid/BT_B2Droid.BT_B2Droid" (Transformation|GetActorLocation (Utilities|Array|Get(acopy) _spawn_points 3)) "0, 0, 0" false 0)
  (AI|SpawnAIFromClass "/Game/Characters/AI_B1Droid/AI_B1Droid.AI_B1Droid_C" "/Game/Characters/AI_B2Droid/BT_B2Droid.BT_B2Droid" (Transformation|GetActorLocation (Utilities|Array|Get(acopy) _spawn_points 4)) "0, 0, 0" false 0)
  (AI|SpawnAIFromClass "/Game/Characters/AI_B1Droid/AI_B1Droid.AI_B1Droid_C" 0 (Transformation|GetActorLocation (Utilities|Array|Get(acopy) _spawn_points 5)) "0, 0, 0" false 0)
  (AI|SpawnAIFromClass "/Game/Characters/AI_B1Droid/AI_B1Droid.AI_B1Droid_C" 0 (Transformation|GetActorLocation (Utilities|Array|Get(acopy) _spawn_points 6)) "0, 0, 0" false 0)
  (Default|StartAIBehaviour (Utilities|Array|Get(acopy) (Variables|Default|GetVulture%20Spawn))))

(fn EnemiesforFirstWave
  (bind _spawn_points (Variables|Default|GetSpawn%20Points))
  (AI|SpawnAIFromClass "/Game/Characters/AI_B2Droid/AI_B2Droid.AI_B2Droid_C" "/Game/Characters/AI_B2Droid/BT_B2Droid.BT_B2Droid" (Transformation|GetActorLocation (Utilities|Array|Get(acopy) _spawn_points)) "0, 0, 0" false 0)
  (AI|SpawnAIFromClass "/Game/Characters/AI_B1Droid/AI_B1Droid.AI_B1Droid_C" 0 (Transformation|GetActorLocation (Utilities|Array|Get(acopy) _spawn_points 1)) "0, 0, 0" false 0)
  (AI|SpawnAIFromClass "/Game/Characters/AI_B1Droid/AI_B1Droid.AI_B1Droid_C" 0 (Transformation|GetActorLocation (Utilities|Array|Get(acopy) _spawn_points 2)) "0, 0, 0" false 0))

(fn StartNewWave
  (bind _result (Math|Integer|IncrementInt (Variables|Default|GetCurrent%20Wave))
    (:%20%20
      (Variables|Default|SetCurrent%20Wave _result)
      (if (== (Variables|Default|GetCurrent%20Wave) 1)
        (Variables|Default|SetEnemies%20Left 3)
        (CallFunction|EnemiesforFirstWave)
        (elif (== (Variables|Default|GetCurrent%20Wave) 2)
          (Variables|Default|SetEnemies%20Left 5)
          (CallFunction|EnemiesforSecondWave)
          (elif (== (Variables|Default|GetCurrent%20Wave) 3)
            (Variables|Default|SetEnemies%20Left 7)
            (CallFunction|EnemiesforThirdWave)
            (elif (== (Variables|Default|GetCurrent%20Wave) 4)
              (Variables|Default|SetEnemies%20Left 6)
              (CallFunction|EnemiesforFourthWave))))))))

(fn EnemiesforFourthWave
  (bind _spawn_points (Variables|Default|GetSpawn%20Points))
  (AI|SpawnAIFromClass "/Game/Characters/AI_B1Droid/AI_B1Droid.AI_B1Droid_C" 0 (Transformation|GetActorLocation (Utilities|Array|Get(acopy) _spawn_points 12)) "0, 0, 0" false 0)
  (AI|SpawnAIFromClass "/Game/Characters/AI_B1Droid/AI_B1Droid.AI_B1Droid_C" 0 (Transformation|GetActorLocation (Utilities|Array|Get(acopy) _spawn_points 13)) "0, 0, 0" false 0)
  (AI|SpawnAIFromClass "/Game/Characters/AI_B2Droid/AI_B2Droid.AI_B2Droid_C" "/Game/Characters/AI_B2Droid/BT_B2Droid.BT_B2Droid" (Transformation|GetActorLocation (Utilities|Array|Get(acopy) _spawn_points 14)) "0, 0, 0" false 0)
  (AI|SpawnAIFromClass "/Game/Characters/AI_B1Droid/AI_B1Droid.AI_B1Droid_C" 0 (Transformation|GetActorLocation (Utilities|Array|Get(acopy) _spawn_points 15)) "0, 0, 0" false 0)
  (AI|SpawnAIFromClass "/Game/Characters/AI_B1Droid/AI_B1Droid.AI_B1Droid_C" 0 (Transformation|GetActorLocation (Utilities|Array|Get(acopy) _spawn_points 16)) "0, 0, 0" false 0)
  (Default|StartAIBehaviour (Utilities|Array|Get(acopy) (Variables|Default|GetVulture%20Spawn) 3)))