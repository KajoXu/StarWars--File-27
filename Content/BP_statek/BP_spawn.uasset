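; Trigger-box spawner that runs a one-time droid encounter and unlocks BP_Doors_2 once the enemy count reaches zero.
; CanGoto sets whether spawning is allowed and resets the count, and the first permitted box overlap calls SpawnEnemies.
; A B1 droid spawns at each spawn point, except a B2 droid with its own behavior tree at the fifth.
; HesDead decrements the count and sets CanOpenDoors at zero.
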(event OnComponentBeginOverlap(Box)
  (params (OverlappedComponent :type Primitive%20Component%20Object%20Reference) (OtherActor :type Actor%20Object%20Reference) (OtherComp :type Primitive%20Component%20Object%20Reference) (OtherBodyIndex :type Integer) (bFromSweep :type Boolean) (SweepResult :type Hit%20Result%20Structure%20%28by%20ref%29))
  (if (Variables|Default|GetCanSpawnEnemies?)
    (Utilities|FlowControl|DoOnce false
      (:Completed
        (CallFunction|SpawnEnemies)))))

(event EventHesDead
  (bind _result (Math|Integer|DecrementInt (Variables|Default|GetEnemies%20Left))
    (:%20%20
      (Variables|Default|SetEnemies%20Left _result)
      (if (== (Variables|Default|GetEnemies%20Left) 0)
        (Variables|/Game/BP_statek/BP_Doors_2.BP_Doors_2_C|SetCan%20Open%20Doors (Variables|Default|Getdoors2%20REF) true)))))

(event EventCanGoto
  (params (CanGoTo? :type Boolean))
  (Variables|Default|SetCanSpawnEnemies? CanGoTo?)
  (Variables|Default|SetEnemies%20Left 5))

(event EventBeginPlay
  (bind _returnvalue (Actor|GetActorOfClass "/Game/BP_statek/BP_Doors_2.BP_Doors_2_C"))
  (Variables|Default|Setdoors2%20REF _returnvalue))

(fn ConstructionScript)

(fn SpawnEnemies
  (for (_array_element _array_index) (Variables|Default|GetSpawn%20Points)
    (if (!= _array_index 4)
      (AI|SpawnAIFromClass "/Game/Characters/AI_B1Droid/AI_B1Droid.AI_B1Droid_C" 0 (Transformation|GetActorLocation _array_element) "0, 0, 0" false 0)
      (else
        (AI|SpawnAIFromClass "/Game/Characters/AI_B2Droid/AI_B2Droid.AI_B2Droid_C" "/Game/Characters/AI_B2Droid/BT_B2Droid.BT_B2Droid" (Transformation|GetActorLocation _array_element) "0, 0, 0" false 0)))))