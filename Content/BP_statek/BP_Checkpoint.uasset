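; BP_Checkpoint is a checkpoint actor that saves the player's respawn or load position when reached.
; An overlap on its CheckpointBox by a BP_twi_lek, gated by the CanGetCheckpoint flag, triggers a one-time save.
; It creates a new BP_Save object, stores the Checkpoint reference's transform as PlayerPos, writes it to a fixed slot and prints a confirmation.
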(event OnComponentBeginOverlap(CheckpointBox)
  (params (OverlappedComponent :type Primitive%20Component%20Object%20Reference) (OtherActor :type Actor%20Object%20Reference) (OtherComp :type Primitive%20Component%20Object%20Reference) (OtherBodyIndex :type Integer) (bFromSweep :type Boolean) (SweepResult :type Hit%20Result%20Structure%20%28by%20ref%29))
  (if (and (== (Utilities|GetClass OtherActor) "/Game/Characters/twi_lek/BP_twi_lek.BP_twi_lek_C") (Variables|Default|GetCanGetCheckpoint))
    (Utilities|FlowControl|DoOnce false
      (:Completed
        (bind _returnvalue (SaveGame|CreateSaveGameObject "/Game/BP_statek/BP_Save.BP_Save_C"))
        (Variables|/Game/BP_statek/BP_Save.BP_Save_C|SetPlayerPos _returnvalue (Transformation|GetActorTransform (Variables|Default|GetCheckpoint)))
        (SaveGame|SaveGametoSlot _returnvalue "save1")
        (Development|PrintString "game saved")))))

(fn ConstructionScript)