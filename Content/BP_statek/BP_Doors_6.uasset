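; Sliding double door Blueprint that opens and closes on events and can also spawn droid enemies.
; OpenDoors plays a timeline that lerps the two door meshes' relative locations between stored old and new positions, and CloseDoors reverses it.
; A separate SpawnEnemies function, not called within this Blueprint, spawns B2 droids with a behavior tree and a B1 droid without one at SpawnPoints actor locations.
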(event Custom|CloseDoors
  (bind _newtrack_0 (Timeline|Timeline_Doors Reverse)
    (:Update
      (Transformation|SetRelativeLocation (Variables|Default|Getdrzwi_drzwi_008) (Math|Vector|Lerp(Vector) (Variables|Default|Getoldr) (Variables|Default|Getnewr) _newtrack_0) false false)
      (Transformation|SetRelativeLocation (Variables|Default|Getdrzwi_drzwi_009) (Math|Vector|Lerp(Vector) (Variables|Default|Getoldl) (Variables|Default|Getnewl) _newtrack_0) false false))))

(event Custom|OpenDoors
  (bind _newtrack_0 (Timeline|Timeline_Doors Play)
    (:Update
      (Transformation|SetRelativeLocation (Variables|Default|Getdrzwi_drzwi_008) (Math|Vector|Lerp(Vector) (Variables|Default|Getoldr) (Variables|Default|Getnewr) _newtrack_0) false false)
      (Transformation|SetRelativeLocation (Variables|Default|Getdrzwi_drzwi_009) (Math|Vector|Lerp(Vector) (Variables|Default|Getoldl) (Variables|Default|Getnewl) _newtrack_0) false false))))

(fn ConstructionScript)

(fn SpawnEnemies
  (bind _spawn_points (Variables|Default|GetSpawn%20Points))
  (AI|SpawnAIFromClass "/Game/Characters/AI_B2Droid/AI_B2Droid.AI_B2Droid_C" "/Game/Characters/AI_B2Droid/BT_B2Droid.BT_B2Droid" (Transformation|GetActorLocation (Utilities|Array|Get(acopy) _spawn_points)) "0, 0, 0" false 0)
  (AI|SpawnAIFromClass "/Game/Characters/AI_B1Droid/AI_B1Droid.AI_B1Droid_C" 0 (Transformation|GetActorLocation (Utilities|Array|Get(acopy) _spawn_points 1)) "0, 0, 0" false 0)
  (AI|SpawnAIFromClass "/Game/Characters/AI_B2Droid/AI_B2Droid.AI_B2Droid_C" "/Game/Characters/AI_B2Droid/BT_B2Droid.BT_B2Droid" (Transformation|GetActorLocation (Utilities|Array|Get(acopy) _spawn_points 2)) "0, 0, 0" false 0))