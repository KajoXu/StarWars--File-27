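; Encounter trigger for a droid fight that opens a BP_Doors_5 door once its enemies are dead.
; The first overlap of its box sets the enemy counter, spawns AI at the SpawnPoints and sets the player BP_twi_lek's Health X to a fixed value.
; Spawns are B1 droids, except one index that gets a B2 droid with its own behavior tree.
; HesDead decrements the counter and opens the door at zero.
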(event OnComponentBeginOverlap(Box)
  (params (OverlappedComponent :type Primitive%20Component%20Object%20Reference) (OtherActor :type Actor%20Object%20Reference) (OtherComp :type Primitive%20Component%20Object%20Reference) (OtherBodyIndex :type Integer) (bFromSweep :type Boolean) (SweepResult :type Hit%20Result%20Structure%20%28by%20ref%29))
  (Utilities|FlowControl|DoOnce false
    (:Completed
      (Variables|Default|SetEnemies%20Left 5)
      (CallFunction|SpawnEnemies)
      (Variables|/Game/Characters/twi_lek/BP_twi_lek.BP_twi_lek_C|SetHealth (stale EventBeginPlay _asbp_twi_lek) (Math|Vector2D|MakeVector2D 5e+02 (.y (Variables|/Game/Characters/twi_lek/BP_twi_lek.BP_twi_lek_C|GetHealth (stale EventBeginPlay _asbp_twi_lek))))))))

(event EventHesDead
  (bind _result (Math|Integer|DecrementInt (Variables|Default|GetEnemies%20Left))
    (:%20%20
      (Variables|Default|SetEnemies%20Left _result)
      (if (== (Variables|Default|GetEnemies%20Left) 0)
        (Default|OpenDoors (Variables|Default|Getdoors5%20REF))))))

(event EventBeginPlay
  (bind _returnvalue (Actor|GetActorOfClass "/Game/BP_statek/BP_Doors_5.BP_Doors_5_C"))
  (Variables|Default|Setdoors5%20REF _returnvalue)
  (bind _asbp_twi_lek (Utilities|Casting|CastToBP_twi_lek (Game|GetPlayerCharacter 0))))

(fn ConstructionScript)

(fn SpawnEnemies
  (for (_array_element _array_index) (Variables|Default|GetSpawn%20Points)
    (if (!= _array_index 4)
      (AI|SpawnAIFromClass "/Game/Characters/AI_B1Droid/AI_B1Droid.AI_B1Droid_C" 0 (Transformation|GetActorLocation _array_element) "0, 0, 0" false 0)
      (else
        (AI|SpawnAIFromClass "/Game/Characters/AI_B2Droid/AI_B2Droid.AI_B2Droid_C" "/Game/Characters/AI_B2Droid/BT_B2Droid.BT_B2Droid" (Transformation|GetActorLocation _array_element) "0, 0, 0" false 0)))))