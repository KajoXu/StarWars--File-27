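; BP_spawn2 is a trigger box that advances the level when the Twi'lek player enters it, switching doors and spawning droid encounters.
; At BeginPlay it caches door, TSERIES and player references.
; A resettable DoOnce picks a branch from the RightDoors and FinalDoors flags: B1 wave, final doors with a TSERIES call, or mixed B1/B2 wave with player health set.
; Both waves spawn at preset points and set a door's EnemiesLeft count.
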(event OnComponentBeginOverlap(Box)
  (params (OverlappedComponent :type Primitive%20Component%20Object%20Reference) (OtherActor :type Actor%20Object%20Reference) (OtherComp :type Primitive%20Component%20Object%20Reference) (OtherBodyIndex :type Integer) (bFromSweep :type Boolean) (SweepResult :type Hit%20Result%20Structure%20%28by%20ref%29))
  (bind _doors6_ref (Variables|Default|Getdoors6%20REF))
  (bind _doors4_ref (Variables|Default|Getdoors4%20REF))
  (if (== (Utilities|GetClass OtherActor) "/Game/Characters/twi_lek/BP_twi_lek.BP_twi_lek_C")
    (Utilities|FlowControl|DoOnce false
      (:Completed
        (if (Variables|Default|GetrightDoors)
          (Default|CloseDoors (Variables|Default|Getdoors5%20REF))
          (Default|OpenDoors _doors6_ref)
          (CallFunction|SpawnEnemies)
          (Variables|/Game/BP_statek/BP_Doors_7.BP_Doors_7_C|SetEnemies%20Left (Utilities|Array|Get(acopy) (stale EventBeginPlay _outactors_4)) 4)
          (elif (Variables|Default|GetfinalDoors?)
            (Default|CloseDoors _doors4_ref)
            (Default|OpenFinalDoors (Variables|Default|Getfinaldoors%20REF))
            (Default|HeIsinTrouble (Variables|Default|GetT-SERIES%20REF))
            (else
              (Default|CloseDoors _doors6_ref)
              (Default|OpenDoors _doors4_ref)
              (CallFunction|SpawnEnemies2)
              (Variables|/Game/BP_statek/BP_Doors_8.BP_Doors_8_C|SetEnemies%20Left (Variables|Default|Getdoors8%20REF) 4)
              (Variables|/Game/Characters/twi_lek/BP_twi_lek.BP_twi_lek_C|SetHealth (Variables|Default|Gettwilek%20REF) "(X=500.000000,Y=500.000000)"))))))))

(event Custom|ResetState
  (bind _doors6_ref (Variables|Default|Getdoors6%20REF))
  (bind _doors4_ref (Variables|Default|Getdoors4%20REF))
  (Utilities|FlowControl|DoOnce false) ; enters at Reset
)

(event EventBeginPlay
  (bind _outactors (Actor|GetAllActorsOfClass "/Game/BP_statek/BP_Doors_4.BP_Doors_4_C"))
  (Variables|Default|Setdoors4%20REF (Utilities|Array|Get(acopy) _outactors))
  (bind _outactors_2 (Actor|GetAllActorsOfClass "/Game/BP_statek/BP_Doors_5.BP_Doors_5_C"))
  (Variables|Default|Setdoors5%20REF (Utilities|Array|Get(acopy) _outactors_2))
  (bind _outactors_3 (Actor|GetAllActorsOfClass "/Game/BP_statek/BP_Doors_6.BP_Doors_6_C"))
  (Variables|Default|Setdoors6%20REF (Utilities|Array|Get(acopy) _outactors_3))
  (bind _outactors_4 (Actor|GetAllActorsOfClass "/Game/BP_statek/BP_Doors_7.BP_Doors_7_C"))
  (bind _outactors_5 (Actor|GetAllActorsOfClass "/Game/BP_statek/BP_Doors_8.BP_Doors_8_C"))
  (Variables|Default|Setdoors8%20REF (Utilities|Array|Get(acopy) _outactors_5))
  (bind _outactors_6 (Actor|GetAllActorsOfClass "/Game/BP_statek/BP_FinalDoors.BP_FinalDoors_C"))
  (Variables|Default|Setfinaldoors%20REF (Utilities|Array|Get(acopy) _outactors_6))
  (bind _returnvalue (Actor|GetActorOfClass "/Game/Characters/T-SERIES/BP_T-SERIES.BP_T-SERIES_C"))
  (Variables|Default|SetT-SERIES%20REF _returnvalue)
  (bind _asbp_twi_lek (Utilities|Casting|CastToBP_twi_lek (Game|GetPlayerCharacter 0)))
  (Variables|Default|Settwilek%20REF _asbp_twi_lek))

(fn ConstructionScript)

(fn SpawnEnemies
  (for _array_element (Variables|Default|GetSpawnPoints)
    (AI|SpawnAIFromClass "/Game/Characters/AI_B1Droid/AI_B1Droid.AI_B1Droid_C" 0 (Transformation|GetActorLocation _array_element) "0, 0, 0" false 0)))

(fn SpawnEnemies2
  (bind _spawnpoints2 (Variables|Default|GetSpawnPoints2))
  (AI|SpawnAIFromClass "/Game/Characters/AI_B1Droid/AI_B1Droid.AI_B1Droid_C" 0 (Transformation|GetActorLocation (Utilities|Array|Get(acopy) _spawnpoints2)) "0, 0, 0" false 0)
  (AI|SpawnAIFromClass "/Game/Characters/AI_B1Droid/AI_B1Droid.AI_B1Droid_C" 0 (Transformation|GetActorLocation (Utilities|Array|Get(acopy) _spawnpoints2 1)) "0, 0, 0" false 0)
  (AI|SpawnAIFromClass "/Game/Characters/AI_B2Droid/AI_B2Droid.AI_B2Droid_C" "/Game/Characters/AI_B2Droid/BT_B2Droid.BT_B2Droid" (Transformation|GetActorLocation (Utilities|Array|Get(acopy) _spawnpoints2 2)) "0, 0, 0" false 0)
  (AI|SpawnAIFromClass "/Game/Characters/AI_B2Droid/AI_B2Droid.AI_B2Droid_C" "/Game/Characters/AI_B2Droid/BT_B2Droid.BT_B2Droid" (Transformation|GetActorLocation (Utilities|Array|Get(acopy) _spawnpoints2 3)) "0, 0, 0" false 0))