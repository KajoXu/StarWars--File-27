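; BP_activeMG is a trigger volume that starts the Magnaguard fight.
; On BeginPlay it caches the first Magnaguard, its AI controller and BP_Doors_8 found in the level.
; When a BP_twi_lek overlaps its box, a DoOnce closes the doors and tells both the Magnaguard and its controller to begin fighting.
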(event OnComponentBeginOverlap(Box)
  (params (OverlappedComponent :type Primitive%20Component%20Object%20Reference) (OtherActor :type Actor%20Object%20Reference) (OtherComp :type Primitive%20Component%20Object%20Reference) (OtherBodyIndex :type Integer) (bFromSweep :type Boolean) (SweepResult :type Hit%20Result%20Structure%20%28by%20ref%29))
  (if (== (Utilities|GetClass OtherActor) "/Game/Characters/twi_lek/BP_twi_lek.BP_twi_lek_C")
    (Utilities|FlowControl|DoOnce false
      (:Completed
        (Default|CloseDoors (Variables|Default|Getdoors8%20REF))
        (Default|StartFight (Variables|Default|GetMG%20REF))
        (Default|StartFighting (Variables|Default|GetMG_C%20REF))))))

(event EventBeginPlay
  (bind _returnvalue (Actor|GetActorOfClass "/Game/Characters/AI_Magnaguard/AI_Magnaguard.AI_Magnaguard_C"))
  (Variables|Default|SetMG%20REF _returnvalue)
  (bind _returnvalue_2 (Actor|GetActorOfClass "/Game/BP_statek/BP_Doors_8.BP_Doors_8_C"))
  (Variables|Default|Setdoors8%20REF _returnvalue_2)
  (bind _returnvalue_3 (Actor|GetActorOfClass "/Game/Characters/AI_Magnaguard/AI_MagnaguardController.AI_MagnaguardController_C"))
  (Variables|Default|SetMG_C%20REF _returnvalue_3))

(fn ConstructionScript)