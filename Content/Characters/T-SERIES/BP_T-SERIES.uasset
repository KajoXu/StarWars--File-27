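; BP_T-SERIES is a character Blueprint that tracks health and plays a death montage when killed.
; Any damage reduces Health, and when it drops below zero the death animation plays on the mesh, followed by a short delay with nothing after it.
; A HeisInTrouble event sets InTrouble and then SurrPLS after timed delays, apparently flagging a trouble and surrender state.
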(event Custom|He%20is%20In%20Trouble
  (Utilities|FlowControl|Delay 2.0)
  (Variables|Default|SetinTrouble? true)
  (Utilities|FlowControl|Delay 1.0)
  (Variables|Default|SetsurrPLS true))

(event Game|Damage|EventAnyDamage
  (params (Damage :type Float%20%28single-precision%29) (DamageType :type Damage%20Type%20Object%20Reference) (InstigatedBy :type Controller%20Object%20Reference) (DamageCauser :type Actor%20Object%20Reference))
  (bind _output_get (Variables|Default|SetHealth (- (Variables|Default|GetHealth) Damage)))
  (if (< _output_get 0.0)
    (Animation|Montage|PlayMontage (Variables|Character|GetMesh) "/Game/Characters/T-SERIES/Animations/T-SERIES_Anim_death_Montage.T-SERIES_Anim_death_Montage"
      (:then
        (Utilities|FlowControl|Delay 2.0)))))

(fn ConstructionScript)